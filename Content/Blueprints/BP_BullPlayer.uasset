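; BP_BullPlayer is a player Blueprint that launches its physics mesh toward the mouse with a hold-and-release charge.
; Each tick, a cursor component follows the deprojected mouse X/Y at the mesh's height, setting the normalized charge direction.
; Enhanced Input builds a clamped charge meter while held; on release, it scales a mass-independent impulse along that direction.
; The meter is never reset here.
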(event `self.ReceiveBeginPlay`
  (`EnhancedInputSubsystemInterface.AddMappingContext` (pcsubsystem `EnhancedInputLocalPlayerSubsystem` (`GameplayStatics.GetPlayerController` 0)) "/Game/Input/IMC_BullPlayer.IMC_BullPlayer" 0 (struct)))

(event `self.ReceiveTick`
  (params (DeltaSeconds :type "Float (single-precision)"))
  (bind _worldlocation (`PlayerController.DeprojectMousePositionToWorld` (`GameplayStatics.GetPlayerController` 0)))
  (bind (_returnvalue_x _returnvalue_y _returnvalue_z) (`KismetMathLibrary.BreakVector` (`SceneComponent.K2_GetComponentLocation` (`self.StaticMesh`))))
  (`SceneComponent.K2_SetWorldLocation` (`self.Cursor`) (`KismetMathLibrary.MakeVector` (.x _worldlocation) (.y _worldlocation) _returnvalue_z) false true)
  (set `self.ChargeDirection` (`KismetMathLibrary.Normal` (- (`SceneComponent.K2_GetComponentLocation` (`self.Cursor`)) (`SceneComponent.K2_GetComponentLocation` (`self.StaticMesh`))))))

(event `EnhancedInput|/Game/Input/IA_Charge`
  (params (ActionValue :type Boolean) (ElapsedSeconds :type "Float (double-precision)") (TriggeredSeconds :type "Float (double-precision)") (InputAction :type "InputAction Object Reference" :default "/Game/Input/IA_Charge.IA_Charge"))
  (:`Triggered`
    ;[1 1 1] Charge meter
    (set `self.ChargeMeter` (`KismetMathLibrary.FClamp` (+ (`self.ChargeMeter`) (* (`self.ChargeRate`) (`GameplayStatics.GetWorldDeltaSeconds`))))))
  (:`Completed`
    ;[1 1 1] Add impulse to ball
    (`PrimitiveComponent.AddImpulse` (`self.StaticMesh`) (* (`self.ChargeDirection`) (* (`self.ChargeImpulse`) (`self.ChargeMeter`))) "None" true)))

(fn `UserConstructionScript`)